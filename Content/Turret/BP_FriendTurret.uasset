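; BP_FriendTurret is a companion turret that glides toward a target point, by default the player character's TurretPos component.
; On BeginPlay it caches that idle point and registers with Mimi_IntroState as a friend.
; Tick interpolates its location and faces the target, which Fetch can replace.
; Disconnected, non-working logic was meant to copy a line-traced material onto its body to fetch a colour.
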(event Custom|Fetch
  (params (Target :type Scene%20Component%20Object%20Reference))
  (Variables|Default|SetTargetPos Target))

(event EventTick
  (params (DeltaSeconds :type Float%20%28single-precision%29))
  (bind _returnvalue (Transformation|GetActorLocation))
  (bind _targetpos (Variables|Default|GetTargetPos))
  (bind _returnvalue_2 (Transformation|GetWorldLocation _targetpos))
  ;[0.15 0.15 0.15 0.5] Move towards the target position
  (Transformation|SetActorLocation (Math|Interpolation|VInterpTo _returnvalue _returnvalue_2 DeltaSeconds (Variables|Default|GetMovementSpeed)) false false)
  (Transformation|SetActorRotation (Math|Rotator|FindLookatRotation _returnvalue _returnvalue_2)))

(event EventBeginPlay
  ;[0.15 0.15 0.15 0.5] Cache variables
  (|CallParentFunction)
  (bind _output_get (Variables|Default|SetTargetPos (Variables|/Game/ThirdPerson/Blueprints/BP_ThirdPersonCharacter.BP_ThirdPersonCharacter_C|GetTurretPos (.AsBP%20Third%20Person%20Character (Utilities|Casting|CastToBP_ThirdPersonCharacter (Game|GetPlayerCharacter 0))))))
  (Variables|Default|SetIdlePos _output_get)
  (bind _asmimi_intro_state (Utilities|Casting|CastToMimi_IntroState (Game|GetGameState)))
  (Default|RegisterFriend _asmimi_intro_state self))

(fn ConstructionScript
  (|CallParentFunction))