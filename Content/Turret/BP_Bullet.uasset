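; Turret bullet actor that, when it hits the player character, reports its Damage to the game state as a resource increment.
; On BeginPlay it caches the Mimi_IntroState game state and starts a LifeTime timer that destroys it.
; Any capsule overlap with another actor also destroys it, but only the player triggers IncrementResource, using a fixed resource type.
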(event OnComponentBeginOverlap(Capsule)
  (params (OverlappedComponent :type Primitive%20Component%20Object%20Reference) (OtherActor :type Actor%20Object%20Reference) (OtherComp :type Primitive%20Component%20Object%20Reference) (OtherBodyIndex :type Integer) (bFromSweep :type Boolean) (SweepResult :type Hit%20Result%20Structure%20%28by%20ref%29))
  (if (!= self OtherActor)
    (Actor|DestroyActor)
    (if (== OtherActor (Game|GetPlayerCharacter 0))
      (Default|IncrementResource (Variables|Default|GetGameState) (Variables|Default|GetDamage) "NewEnumerator1"))))

(event Custom|SelfDestruct
  (Actor|DestroyActor))

(event EventBeginPlay
  (Utilities|Time|SetTimerbyEvent (delegate Custom|SelfDestruct) (Variables|Default|GetLifeTime))
  (bind _asmimi_intro_state (Utilities|Casting|CastToMimi_IntroState (Game|GetGameState)))
  (Variables|Default|SetGameState _asmimi_intro_state))

(fn ConstructionScript)