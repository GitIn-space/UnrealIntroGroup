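; BP_ButtonKey is a coin-gated button that charges the player to open a door.
; On Activate, while active, it reads CoinsPickedUp from the Mimi_IntroState game state and compares it to KeyRequired.
; With enough coins it deducts the cost, fires ButtonActivated and deactivates itself; otherwise it prints how many are missing.
; The Key-named variables actually count coins, and player feedback is through PrintString only.
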(event EventActivate
  ;[0.15 0.15 0.15 0.5] Button is pressed and makes sure you have enough money.
  ; And then takes the amount of money needed.
  ; The door then opens.
  (if (Variables|Default|GetIs%20Active)
    (Development|PrintString "Button be bressed")
    (CallFunction|EvaluateCoins)))

(fn ConstructionScript)

(fn EvaluateCoins
  (Variables|Default|SetKey%20Collected%20Ref (Variables|/Game/MimiMapp/Saker/EgnaBluePrints/Mimi_IntroState.Mimi_IntroState_C|GetCoins%20picked%20up (.AsMimi%20Intro%20State (Utilities|Casting|CastToMimi_IntroState (Game|GetGameState)))))
  (if (<= (Variables|Default|GetKeyRequired) (Variables|Default|GetKey%20Collected%20Ref))
    (Variables|/Game/MimiMapp/Saker/EgnaBluePrints/Mimi_IntroState.Mimi_IntroState_C|SetCoins%20picked%20up (.AsMimi%20Intro%20State (Utilities|Casting|CastToMimi_IntroState (Game|GetGameState))) (- (Variables|Default|GetKey%20Collected%20Ref) (Variables|Default|GetKeyRequired)))
    (Development|PrintString "The door is now open. :)" :!label _label)
    (Default|CallButtonActivated)
    (Variables|Default|SetIs%20Active false)
    (else
      (bind _output_get (Variables|Default|SetHow%20many%20keys%20needed (- (Variables|Default|GetKeyRequired) (Variables|Default|GetKey%20Collected%20Ref))))
      (if (== _output_get 0)
        (goto _label)
        (else
          (Development|PrintString (Utilities|String|ToString(Text) (Utilities|Text|FormatText "You're missing {coins}..." (Variables|Default|GetHow%20many%20keys%20needed)))))))))