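; BP_YouWinnable is a win trigger actor that sends the player to the victory screen on touch.
; When its Collider begins overlapping the player character, it opens the Map_WinScreen level.
; The construction script applies a configurable static mesh and material to its Triangle component, so each placed instance can set its own look.
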(event OnComponentBeginOverlap(Collider)
  (params (OverlappedComponent :type Primitive%20Component%20Object%20Reference) (OtherActor :type Actor%20Object%20Reference) (OtherComp :type Primitive%20Component%20Object%20Reference) (OtherBodyIndex :type Integer) (bFromSweep :type Boolean) (SweepResult :type Hit%20Result%20Structure%20%28by%20ref%29))
  ;[0.15 0.15 0.15 0.5] Colliding with this object sends you to the win screen.
  ;;[0.15 0.15 0.15 0.5] Only when colliding with the player
  (if (== OtherActor (Game|GetPlayerCharacter 0))
    (Game|OpenLevel(byName) "Map_WinScreen")))

(event EventBeginPlay)

(event Collision|EventActorBeginOverlap
  (params (OtherActor :type Actor%20Object%20Reference)))

(event EventTick
  (params (DeltaSeconds :type Float%20%28single-precision%29)))

(fn ConstructionScript
  (Components|StaticMesh|SetStaticMesh (Variables|Default|GetTriangle) (Variables|Default|GetStatic%20mesh))
  (Rendering|Material|SetMaterial (Variables|Default|GetTriangle) 0 (Variables|Default|GetMaterial)))