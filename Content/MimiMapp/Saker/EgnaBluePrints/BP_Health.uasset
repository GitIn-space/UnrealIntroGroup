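; BP_Health is a configurable pickup actor that adds to a resource when the player collects it.
; The construction script applies the chosen mesh and material to its Sphere component.
; When the player character overlaps the Collider, it spawns a pickup sound and particle effect, passes its amount and type to IncrementResource on the Mimi_IntroState game state, then destroys itself.
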(event OnComponentBeginOverlap(Collider)
  (params (OverlappedComponent :type Primitive%20Component%20Object%20Reference) (OtherActor :type Actor%20Object%20Reference) (OtherComp :type Primitive%20Component%20Object%20Reference) (OtherBodyIndex :type Integer) (bFromSweep :type Boolean) (SweepResult :type Hit%20Result%20Structure%20%28by%20ref%29))
  (bind _self self)
  (bind _returnvalue (Transformation|GetActorLocation _self))
  ;[0.15 0.15 0.15 0.5] Coin gets destroyed when colliding with the player
  (if (== OtherActor (Game|GetPlayerCharacter 0))
    (Utilities|FlowControl|Sequence
      (:then_1
        (Audio|SpawnSoundatLocation (Variables|Default|GetPick%20up%20Sound) _returnvalue "0, 0, 0" 1.0 1.0 0.0 0 0))
      (:then_2
        (Effects|SpawnEmitteratLocation (Variables|Default|GetPick%20up%20Particle) _returnvalue))
      (:then_3
        (Default|IncrementResource (.AsMimi%20Intro%20State (Utilities|Casting|CastToMimi_IntroState (Game|GetGameState))) (Variables|Default|GetAmount%20Collected) (Variables|Default|GetPickable%20Type)))
      (:then_4
        (Actor|DestroyActor)))))

(event EventBeginPlay)

(event Collision|EventActorBeginOverlap
  (params (OtherActor :type Actor%20Object%20Reference)))

(event EventTick
  (params (DeltaSeconds :type Float%20%28single-precision%29)))

(fn ConstructionScript
  (Components|StaticMesh|SetStaticMesh (Variables|Default|GetSphere) (Variables|Default|GetStatic%20mesh))
  (Rendering|Material|SetMaterial (Variables|Default|GetSphere) 0 (Variables|Default|GetMaterial)))