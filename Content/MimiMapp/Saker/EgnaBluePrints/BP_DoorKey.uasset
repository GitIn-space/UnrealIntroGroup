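; BP_DoorKey is a double sliding door linked to a button.
; BeginPlay stores both panels' starting relative locations and binds an event to the button's activation.
; DoorOpen plays a timeline that lerps the panels apart along local Y by OffsetY in opposite directions, and CloseDoor reverses the same timeline to bring them back.
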(event Custom|DoorOpen
  (bind _doorleftorigin (Variables|Default|GetDoorLeftOrigin))
  (bind _doorrightorigin (Variables|Default|GetDoorRightOrigin))
  ;[0.15 0.15 0.15 0.5] Door opening script
  (bind _opendoortrack (Timeline|DoorOpening Play)
    (:Update
      (Transformation|SetRelativeLocation (Variables|Default|GetDoorRight) (Math|Vector|Lerp(Vector) (Variables|Default|GetDoorRightOrigin) (Math|Vector|MakeVector (.x _doorrightorigin) (+ (.y _doorrightorigin) (* (Variables|Default|GetOffsetY) -1.0)) (.z _doorrightorigin)) _opendoortrack) false false)
      (Transformation|SetRelativeLocation (Variables|Default|GetDoorLeft) (Math|Vector|Lerp(Vector) (Variables|Default|GetDoorLeftOrigin) (Math|Vector|MakeVector (.x _doorleftorigin) (+ (.y _doorleftorigin) (Variables|Default|GetOffsetY)) (.z _doorleftorigin)) _opendoortrack) false false))))

(event Custom|CloseDoor
  (bind _doorleftorigin (Variables|Default|GetDoorLeftOrigin))
  (bind _doorrightorigin (Variables|Default|GetDoorRightOrigin))
  ;[0.15 0.15 0.15 0.5] Door opening script
  (bind _opendoortrack (Timeline|DoorOpening Reverse)
    (:Update
      (Transformation|SetRelativeLocation (Variables|Default|GetDoorRight) (Math|Vector|Lerp(Vector) (Variables|Default|GetDoorRightOrigin) (Math|Vector|MakeVector (.x _doorrightorigin) (+ (.y _doorrightorigin) (* (Variables|Default|GetOffsetY) -1.0)) (.z _doorrightorigin)) _opendoortrack) false false)
      (Transformation|SetRelativeLocation (Variables|Default|GetDoorLeft) (Math|Vector|Lerp(Vector) (Variables|Default|GetDoorLeftOrigin) (Math|Vector|MakeVector (.x _doorleftorigin) (+ (.y _doorleftorigin) (Variables|Default|GetOffsetY)) (.z _doorleftorigin)) _opendoortrack) false false))))

(event EventBeginPlay
  (Variables|Default|SetDoorRightOrigin (Variables|/Script/Engine.SceneComponent|GetRelativeLocation (Variables|Default|GetDoorRight)))
  (Variables|Default|SetDoorLeftOrigin (Variables|/Script/Engine.SceneComponent|GetRelativeLocation (Variables|Default|GetDoorLeft)))
  (EventDispatchers|BindEventtoButtonActivated (Variables|Default|GetButton) (EventDispatchers|CreateEvent :!event Custom|DoorOpen)))

(fn ConstructionScript)