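; BP_Checkpoint is a placed checkpoint that records the player's respawn point in the game state.
; When the player character overlaps its Collider, it passes its order number and the RespawnPoint component's world location to SetLastCheckpoint.
; BeginPlay casts the game state to Mimi_IntroState once and caches it for those overlap calls.
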(event OnComponentBeginOverlap(Collider)
  (params (OverlappedComponent :type Primitive%20Component%20Object%20Reference) (OtherActor :type Actor%20Object%20Reference) (OtherComp :type Primitive%20Component%20Object%20Reference) (OtherBodyIndex :type Integer) (bFromSweep :type Boolean) (SweepResult :type Hit%20Result%20Structure%20%28by%20ref%29))
  ;[0.15 0.15 0.15 0.5] Update checkpoint in game state
  (if (== OtherActor (Game|GetPlayerCharacter 0))
    (Default|SetLastCheckpoint (Variables|Default|GetGameState) (Variables|Default|GetNumberInOrder) (Transformation|GetWorldLocation (Variables|Default|GetRespawnPoint)))))

(event EventBeginPlay
  ;[0.15 0.15 0.15 0.5] Cache game state to avoid unnecessary casts
  (bind _asmimi_intro_state (Utilities|Casting|CastToMimi_IntroState (Game|GetGameState)))
  (Variables|Default|SetGameState _asmimi_intro_state))

(fn ConstructionScript)